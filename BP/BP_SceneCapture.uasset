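; BP_SceneCapture is a Blueprint that provides a scene capture feeding the RT_SceneCap render target.
; On BeginPlay it spawns a SceneCapture2D at a fixed world transform if none is set, stores it and assigns the render target to its capture component.
; EndPlay destroys the capture actor, and pressing C only prints a test message.
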(event `self.ReceiveBeginPlay`
  (`/Engine/EditorBlueprintResources/StandardMacros.IsValid` (`self.SceneCap2D`)
    (:`Is Not Valid`
      (bind _returnvalue (`|SpawnActorFromClass` "/Script/Engine.SceneCapture2D" (`KismetMathLibrary.MakeTransform` (1000.0 1000.0 400.0)) "Undefined" "MultiplyWithRoot" null null))
      (bind _output_get (set `self.SceneCap2D` _returnvalue))
      (set `SceneCaptureComponent2D.TextureTarget` "/Game/RT/RT_SceneCap.RT_SceneCap" (`SceneCapture2D.CaptureComponent2D` _output_get)))))

(event `self.ReceiveEndPlay`
  (params (EndPlayReason :type "EEndPlayReason Enum" :default "Destroyed"))
  (`self.K2_DestroyActor` (`self.SceneCap2D`)))

(event `Key|C`
  (params (Key :type "Key Structure"))
  (:`Pressed`
    (`KismetSystemLibrary.PrintString` "Hello")))

(fn `UserConstructionScript`)