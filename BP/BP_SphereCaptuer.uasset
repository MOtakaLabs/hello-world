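; Actor that photographs its origin from viewpoints on a surrounding dome and saves numbered JPGs to the project's Saved directory.
; BeginPlay builds staggered latitude rings plus a top point, triangle indices for a debug wireframe, and a spawned SceneCapture2D targeting a render target.
; Tick draws the wireframe and aims camera and capture inward at each point for 30 frames, exporting on the last.
; Exporting continues after the final point.
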(event `self.ReceiveBeginPlay`
  (bind (_tempvec_x _tempvec_y _tempvec_z) (`KismetMathLibrary.BreakVector` (`self.tempVec`)))
  (bind _indexarray (`self.IndexArray`))
  (bind _segments (`self.segments`))
  (bind _segments_2 (`self.segments`))
  (bind _output (`|GetArrayItem` (`self.pointArray`)))
  (bind _returnvalue (/ 360.0 (`KismetMathLibrary.Conv_IntToDouble` _segments)))
  (`|ExecutionSequence`
    (:`then_0`
      (for _index (range (`self.HeightDiv`))
        (set `self.localOffset` _index)
        (set `self.tempVec` (`KismetMathLibrary.TransformDirection` (`KismetMathLibrary.MakeTransform` (0.0 0.0 0.0) (`KismetMathLibrary.MakeRotator` (* _index (/ -90.0 (`KismetMathLibrary.Conv_IntToDouble` (`self.HeightDiv`)))))) (`KismetMathLibrary.MakeVector` 0.0 (`self.Raduas`))))
        (for _index_2 (range _segments)
          (bind (_returnvalue_x _returnvalue_y) (`KismetMathLibrary.BreakVector` (`KismetMathLibrary.TransformDirection` (`KismetMathLibrary.MakeTransform` (0.0 0.0 0.0) (`KismetMathLibrary.MakeRotator` 0.0 0.0 (+ (* _index_2 _returnvalue) (* (/ _returnvalue 2.0) (`self.localOffset`))))) (`KismetMathLibrary.MakeVector` 0.0 _tempvec_y))))
          (`KismetArrayLibrary.Array_AddUnique` (`self.pointArray`) (+ (`self.K2_GetActorLocation`) (`KismetMathLibrary.MakeVector` _returnvalue_x _returnvalue_y _tempvec_z)))))
      (`KismetArrayLibrary.Array_AddUnique` (`self.pointArray`) (+ (`self.K2_GetActorLocation`) (`KismetMathLibrary.MakeVector` 0.0 0.0 (`self.Raduas`)))))
    (:`then_1`
      (`KismetArrayLibrary.Array_Clear` (`self.IndexArray`))
      (for _index_3 (range (+ (- (`KismetArrayLibrary.Array_Length` (`self.pointArray`)) 2) 1))
        (`KismetArrayLibrary.Array_Add` _indexarray _index_3)
        (`KismetArrayLibrary.Array_Add` _indexarray (+ (mod (+ _index_3 1) _segments_2) (* (/ _index_3 _segments_2) _segments_2)))
        (bind _newindex (`self.CalcuIndex` (+ _index_3 _segments_2)))
        (`KismetArrayLibrary.Array_Add` _indexarray _newindex)))
    (:`then_2`
      (bind _returnvalue_2 (`|SpawnActorFromClass` "/Script/Engine.SceneCapture2D" (`KismetMathLibrary.MakeTransform` _output (`KismetMathLibrary.FindLookAtRotation` _output (`SceneComponent.K2_GetComponentLocation` (`self.DefaultSceneRoot`)))) "AlwaysSpawn" "MultiplyWithRoot" null null))
      (bind _output_get (set `self.SceneCap2D` _returnvalue_2))
      (set `SceneCaptureComponent2D.TextureTarget` "/Game/RT/NewTextureRenderTarget2D.NewTextureRenderTarget2D" (`SceneCapture2D.CaptureComponent2D` _output_get)))
    (:`then_3`
      (set `self.counter` 0))))

(event `self.ReceiveTick`
  (params (DeltaSeconds :type "Float (single-precision)"))
  (bind _camera (`self.Camera`))
  (bind _scenecap2d (`self.SceneCap2D`))
  (bind _output (`|GetArrayItem` (`self.pointArray`) (/ (`self.counter`) 30)))
  (bind _returnvalue (`KismetMathLibrary.FindLookAtRotation` _output (`SceneComponent.K2_GetComponentLocation` (`self.DefaultSceneRoot`))))
  (`|ExecutionSequence`
    (:`then_0`
      (`self.DebugDrawFrame`))
    (:`then_1`
      (if (< (/ (`self.counter`) 30) (`KismetArrayLibrary.Array_Length` (`self.pointArray`)))
        (`SceneComponent.K2_SetWorldLocation` _camera _output false true)
        (`SceneComponent.K2_SetWorldRotation` _camera _returnvalue false false)
        (`self.K2_SetActorLocation` _scenecap2d _output false true)
        (`self.K2_SetActorRotation` _scenecap2d _returnvalue false)))
    (:`then_2`
      (if (== (mod (`self.counter`) 30) 29)
        (`self.SaveImage` null "Capture")
        (`KismetSystemLibrary.PrintString` (`KismetStringLibrary.Conv_IntToString` (`self.CaptureNumber`)))))
    (:`then_3`
      (`/Engine/EditorBlueprintResources/StandardMacros.IncrementInt` (`self.counter`)))))

(fn `CalcuIndex`
  (params (index :type Integer))
  (returns (newIndex :type Integer))
  (locals (NewLocalVar :type Integer :default 0))
  (bind _returnvalue (`KismetArrayLibrary.Array_Length` (`self.pointArray`)))
  (if (>= index _returnvalue)
    (set `local.NewLocalVar` (- _returnvalue 1))
    (else
      (set `local.NewLocalVar` index)))
  (return (`local.NewLocalVar`)))

(fn `DebugDrawFrame`
  (bind _pointarray (`self.pointArray`))
  (bind _indexarray (`self.IndexArray`))
  (for _index (range (/ (`KismetArrayLibrary.Array_Length` (`self.IndexArray`)) 3))
    (bind _returnvalue (* _index 3))
    (bind _output (`|GetArrayItem` _pointarray (`|GetArrayItem` _indexarray _returnvalue)))
    (bind _output_2 (`|GetArrayItem` _pointarray (`|GetArrayItem` _indexarray (+ _returnvalue 1))))
    (`KismetSystemLibrary.DrawDebugLine` _output _output_2 (struct :`G` 1.0 :`B` 0.021 :`A` 1.0) 1.0)
    (bind _output_3 (`|GetArrayItem` _pointarray (`|GetArrayItem` _indexarray (+ _returnvalue 2))))
    (`KismetSystemLibrary.DrawDebugLine` _output_2 _output_3 (struct :`G` 1.0 :`B` 0.021 :`A` 1.0) 1.0)
    (`KismetSystemLibrary.DrawDebugLine` _output_3 _output (struct :`G` 1.0 :`B` 0.021 :`A` 1.0) 1.0)))

(fn `SaveImage`
  (params (Texture :type "Texture Object Reference") (B :type String))
  (`ImageWriteBlueprintLibrary.ExportToDisk` "/Game/RT/NewTextureRenderTarget2D.NewTextureRenderTarget2D" (`KismetStringLibrary.Concat_StrStr` (`KismetSystemLibrary.GetProjectSavedDirectory`) B (`KismetStringLibrary.Conv_IntToString` (`self.CaptureNumber`))) (make `ImageWriteOptions` "JPG"))
  (`/Engine/EditorBlueprintResources/StandardMacros.IncrementInt` (`self.CaptureNumber`)))

(fn `UserConstructionScript`)